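; Player controller for the board game's game room that loads the saved user profile, sets up the player and handles chat.
; On local BeginPlay it reads UserInfo from the save slot and passes it to GameRoomMode_BP to respawn the named character, then creates the room UI.
; Chat messages are relayed through the game mode's controller list, with each controller updating its own chat window widget.
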(event Custom|Pass%20Character%20Info%20to%20Server
  (params (User%20Info :type User%20Info%20STR%20Structure))
  ;[1 1 1] Setup Player
  (Variables|Default|SetUser%20Info User%20Info)
  (bind _asgame_room_mode_bp (Utilities|Casting|CastToGameRoomMode_BP (Game|GetGameMode)))
  (Default|RespawnPlayer _asgame_room_mode_bp self (Utilities|Struct|BreakUserInfo_STR (Variables|Default|GetUser%20Info)))
  (CallFunction|SetupInterface))

(event Custom|Setup%20Interface
  ;[1 1 1] Setup Player
  (bind _returnvalue (UserInterface|CreateWidget "/Game/BoardgameInterface/Environment/GameRoom/GameRoomUI_W.GameRoomUI_W_C"))
  (bind _output_get (Variables|Default|SetGame%20Interface _returnvalue))
  (UserInterface|Viewport|AddtoViewport _output_get 0))

(event Custom|Get%20Chat%20Message
  (params (Text%20to%20Send :type Text))
  ;[1 1 1] Chat
  (Variables|Default|SetSender%20Text Text%20to%20Send)
  (Variables|Default|SetSender%20Name (Utilities|Text|ToText(String) (.CharacterName (Utilities|Struct|BreakUserInfo_STR (Variables|Default|GetUser%20Info)))))
  (bind _asgame_room_mode_bp (Utilities|Casting|CastToGameRoomMode_BP (Game|GetGameMode)))
  (for _array_element (Variables|/Game/BoardgameInterface/Environment/GameRoom/GameRoomMode_BP.GameRoomMode_BP_C|GetUser%20Controllers _asgame_room_mode_bp)
    (bind _asgame_room_controller_bp (Utilities|Casting|CastToGameRoomController_BP _array_element))
    (CallFunction|UpdateChat _asgame_room_controller_bp (Variables|Default|GetSender%20Name) (Variables|Default|GetSender%20Text))))

(event Custom|Update%20Chat
  (params (Sender :type Text) (Text :type Text))
  ;[1 1 1] Chat
  (Default|UpdateChatWindow (Variables|/Game/BoardgameInterface/Environment/GameRoom/GameRoomUI_W.GameRoomUI_W_C|GetUserChatWindow_W_56 (Variables|Default|GetGame%20Interface)) Sender Text))

(event EventBeginPlay
  ;[1 1 1] Load player information.
  (Variables|Default|SetbShowMouseCursor true)
  (if (Pawn|IsLocalController)
    (Viewport|RemoveAllWidgets)
    (CallFunction|LoadGame)
    (CallFunction|PassCharacterInfotoServer (Variables|Default|GetUser%20Info))))

(fn ConstructionScript)

(fn LoadGame
  (bind _returnvalue (SaveGame|LoadGamefromSlot (Variables|/Game/BoardgameInterface/Core/Framework/AppInstance_BP.AppInstance_BP_C|GetSave%20Slot%20Name (.AsApp%20Instance%20BP (Utilities|Casting|CastToAppInstance_BP (Game|GetGameInstance))))))
  (bind _asuser_save_game (Utilities|Casting|CastToUserSaveGame _returnvalue))
  (Variables|Default|SetUser%20Info (Variables|/Game/BoardgameInterface/Core/Framework/UserSaveGame.UserSaveGame_C|GetUser%20Info _asuser_save_game)))