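; Base die actor for the board game room that can be carried under the mouse cursor and thrown with physics.
; While attached, Tick traces from the cursor and hovers the die above the hit point; first attach scales it in.
; Release enables physics and adds a radial impulse based on velocity.
; When the mesh sleeps, ReportResult, which reads no face value here, reverses the scale timeline and destroys the actor.
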(event OnComponentSleep(StaticMesh)
  (params (SleepingComponent :type Primitive%20Component%20Object%20Reference) (BoneName :type Name :default "None"))
  (if (Variables|Default|GetWaiting%20for%20Result)
    (Variables|Default|SetWaiting%20for%20Result false)
    (CallFunction|ReportResult)))

(event Custom|Animate%20In
  (bind (_direction _scale) (Timeline|Animate PlayFromStart)
    (:Update
      (Transformation|SetActorScale3D (Math|Conversions|ToVector(Float) _scale)))
    (:Finished
      (if (Utilities|Enum|Equal(Enum) _direction "Backward")
        (Actor|DestroyActor)))))

(event Custom|Report%20Result
  (CallFunction|AnimateOut))

(event Custom|Animate%20Out
  (bind (_direction _scale) (Timeline|Animate ReverseFromEnd)
    (:Update
      (Transformation|SetActorScale3D (Math|Conversions|ToVector(Float) _scale)))
    (:Finished
      (if (Utilities|Enum|Equal(Enum) _direction "Backward")
        (Actor|DestroyActor)))))

(event EventBeginPlay)

(event EventTick
  (params (DeltaSeconds :type Float%20%28single-precision%29))
  (bind _controller (Variables|Default|GetController))
  (bind (_locationx _locationy) (Game|Player|GetMousePosition _controller))
  (bind (_worldposition _worlddirection) (Class|GameplayStatics|DeprojectScreentoWorld _controller (Math|Vector2D|MakeVector2D _locationx _locationy)))
  (bind _outhit (Collision|LineTraceByChannel _worldposition (+ _worldposition (* _worlddirection 1e+03)) "TraceTypeQuery1" false 0 "None"))
  (Transformation|SetActorLocation (Math|Vector|MakeVector (.x (.ImpactPoint (Collision|BreakHitResult _outhit))) (.y (.ImpactPoint (Collision|BreakHitResult _outhit))) (+ (.z (.ImpactPoint (Collision|BreakHitResult _outhit))) (Variables|Default|GetFloating%20Height))) true false))

(fn ConstructionScript)

(fn AttachtoMouse
  (params (Attached :type Boolean))
  (bind _staticmesh (Variables|Default|GetStaticMesh))
  (bind _returnvalue (Transformation|GetWorldLocation _staticmesh))
  (if Attached
    (Physics|SetSimulatePhysics (Variables|Default|GetStaticMesh) false)
    (Actor|Tick|SetActorTickEnabled true)
    (Variables|Default|SetCurrent%20Time%20to%20Despawn (Variables|Default|GetTime%20to%20Despawn))
    (Variables|Default|SetWaiting%20for%20Result false)
    (if (not (Variables|Default|GetAnimated%20In))
      (Variables|Default|SetAnimated%20In true)
      (CallFunction|Animatein))
    (else
      (Physics|SetSimulatePhysics (Variables|Default|GetStaticMesh) true)
      (Actor|Tick|SetActorTickEnabled false)
      (Variables|Default|SetWaiting%20for%20Result true)
      (bind _returnvalue_2 (Physics|GetPhysicsLinearVelocity _staticmesh "None"))
      (Physics|AddRadialForce _staticmesh (select (<= (Math|Vector|VectorLength _returnvalue_2) 2.0) (+ _returnvalue "0, 0,-10.000000") (+ (* _returnvalue_2 -1.0) _returnvalue)) 1e+01 (select (<= (Math|Vector|VectorLength _returnvalue_2) 2.0) 4e+04 (Math|Random|RandomFloatinRange 2e+04 8e+04)) "RIF_Constant" true))))