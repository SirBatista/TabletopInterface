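; GameRoomPawn_BP is the player pawn for the board game's game room, turning mouse clicks into spawned dice.
; On BeginPlay it caches the GameRoomController_BP, shows the cursor and sets Game and UI input focused on the controller's GameInterface widget.
; The Click action deprojects the mouse position, line traces on Visibility and spawns a scaled-down DiceMaster_BP just above the hit point.
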(event EventBeginPlay
  (|CallParentFunction)
  (bind _asgame_room_controller_bp (Utilities|Casting|CastToGameRoomController_BP (Game|GetPlayerController 0)))
  (bind _output_get (Variables|Default|SetPlayer%20Controller _asgame_room_controller_bp))
  (Variables|/Script/Engine.PlayerController|SetbShowMouseCursor _output_get true)
  (Input|SetInputModeGameandUI _output_get (Variables|/Game/BoardgameInterface/Environment/GameRoom/GameRoomController_BP.GameRoomController_BP_C|GetGame%20Interface _output_get) "DoNotLock" false))

(event Input|ActionEvents|InputActionClick
  (params (Key :type Key%20Structure :default "None"))
  (bind _player_controller (Variables|Default|GetPlayer%20Controller))
  (bind (_locationx _locationy) (Game|Player|GetMousePosition _player_controller))
  (bind (_worldposition _worlddirection) (Class|GameplayStatics|DeprojectScreentoWorld _player_controller (Math|Vector2D|MakeVector2D _locationx _locationy)))
  (:Pressed
    (bind (_outhit _returnvalue) (Collision|LineTraceByChannel _worldposition (+ _worldposition (* _worlddirection 1e+03)) "TraceTypeQuery1" false 0 "None"))
    (if _returnvalue
      (Game|SpawnActorfromClass "/Game/BoardgameInterface/Environment/GameRoom/Assets/3DTray/Dice/DiceMaster_BP.DiceMaster_BP_C" (Math|Transform|MakeTransform (Math|Vector|MakeVector (.x (.ImpactPoint (Collision|BreakHitResult _outhit))) (.y (.ImpactPoint (Collision|BreakHitResult _outhit))) (+ (.z (.ImpactPoint (Collision|BreakHitResult _outhit))) 1e+01)) "0, 0, 0" "0.100000,0.100000,0.100000") "Undefined" 0 0))))

(fn ConstructionScript
  (|CallParentFunction))