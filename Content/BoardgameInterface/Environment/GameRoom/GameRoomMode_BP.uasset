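; Game mode for the board game's game room, handling player controller tracking, pawn spawning and logout.
; It records controllers arriving through controller swaps in a UserControllers list.
; RespawnPlayer destroys any controlled pawn, then spawns and possesses a new GameRoomPawn_BP, leaving its CharacterName input unused.
; On logout, it passes an exiting GameRoomController_BP to the app instance's DestroySessionCaller.
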(event Custom|Respawn%20Player
  (params (Player%20Controller :type Player%20Controller%20Object%20Reference) (Character%20Name :type String))
  (bind _returnvalue (Pawn|GetControlledPawn Player%20Controller))
  ;[1 1 1] Spawn Player
  (Utilities|IsValid _returnvalue
    (:Is%20Valid
      (Actor|DestroyActor _returnvalue))
    (:Is%20Not%20Valid
      _))
  (bind _returnvalue_2 (Game|SpawnActorfromClass "/Game/BoardgameInterface/Environment/GameRoom/GameRoomPawn_BP.GameRoomPawn_BP_C" (Math|Transform|MakeTransform "0, 0, 0" "0, 0, 0" "1,1,1") "Undefined" 0 0))
  (Pawn|Possess Player%20Controller _returnvalue_2))

(event EventOnSwapPlayerControllers
  (params (OldPC :type Player%20Controller%20Object%20Reference) (NewPC :type Player%20Controller%20Object%20Reference))
  ;[1 1 1] Keep track of all new controllers.
  (Utilities|Array|Add (Variables|Default|GetUser%20Controllers) NewPC))

(event EventOnLogout
  (params (ExitingController :type Controller%20Object%20Reference))
  ;[1 1 1] Logout
  (bind _asgame_room_controller_bp (Utilities|Casting|CastToGameRoomController_BP ExitingController))
  (Default|DestroySessionCaller (.AsApp%20Instance%20BP (Utilities|Casting|CastToAppInstance_BP (Game|GetGameInstance))) _asgame_room_controller_bp))

(fn ConstructionScript)