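; Player controller for the board game's multiplayer waiting room, driving the lobby widget, character selection, chat, loading screen and kick or session teardown.
; It loads and saves user info through a save slot, then passes it to WaitingRoomMode_BP, which swaps characters and updates all users.
; Character picks update the game mode's availability array, while update events refresh the user list, map details and buttons.
; Chat fans out through every controller the game mode holds.
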(event Custom|Initial%20Setup
  ;[1 1 1] Initial Setup
  (CallFunction|SaveGameCheck)
  (CallFunction|CallUpdate (Variables|UserInfo|GetUser%20Settings) false))

(event Custom|Call%20Update
  (params (User%20Info :type User%20Info%20STR%20Structure) (Changed%20Status :type Boolean))
  (bind _returnvalue (Game|GetGameMode))
  (bind _aswaiting_room_mode_bp (Utilities|Casting|CastToWaitingRoomMode_BP _returnvalue))
  ;[1 1 1] Update Waiting Room Information
  (Variables|UserInfo|SetUser%20Settings User%20Info)
  (Default|SwapCharacter _aswaiting_room_mode_bp self (Utilities|Struct|BreakUserInfo_STR (Variables|UserInfo|GetUser%20Settings)) Changed%20Status)
  (Default|AllUsersUpdate _aswaiting_room_mode_bp))

(event Custom|Assign%20Player
  (params (Character%20Name :type String) (Character%20Image :type Texture%202D%20Object%20Reference))
  ;[1 1 1] Assigns Selected Character
  (Utilities|Struct|SetmembersinUserInfo_STR (Variables|UserInfo|GetUser%20Settings) Character%20Name Character%20Image)
  (CallFunction|SaveGame)
  (CallFunction|CallUpdate (Variables|UserInfo|GetUser%20Settings) false))

(event Custom|Get%20Chat%20Message
  (params (Text%20to%20Send :type Text))
  ;[1 1 1] Chat Message Replication
  (Variables|UserInfo|SetSender%20Text Text%20to%20Send)
  (Variables|UserInfo|SetSender%20Name (Utilities|Struct|BreakUserInfo_STR (Variables|UserInfo|GetUser%20Settings)))
  (bind _aswaiting_room_mode_bp (Utilities|Casting|CastToWaitingRoomMode_BP (Game|GetGameMode)))
  (for _array_element (Variables|/Game/BoardgameInterface/Environment/WaitingRoom/Framework/WaitingRoomMode_BP.WaitingRoomMode_BP_C|GetUser%20Controllers _aswaiting_room_mode_bp)
    (bind _aswaiting_room_controller_bp (Utilities|Casting|CastToWaitingRoomController_BP _array_element))
    (CallFunction|UpdateChat _aswaiting_room_controller_bp (Utilities|Text|ToText(String) (Variables|UserInfo|GetSender%20Name)) (Variables|UserInfo|GetSender%20Text))))

(event Custom|Update%20Chat
  (params (Sender :type Text) (Text :type Text))
  ;[1 1 1] Updates the Chat Display
  (Default|UpdateChatWindow (Variables|/Game/BoardgameInterface/Environment/WaitingRoom/WaitingRoom_W.WaitingRoom_W_C|GetUserChatWindow_W (Variables|Widgets|GetWaiting%20Room%20Menu)) Sender Text))

(event Custom|Setup%20Lobby%20Menu
  (params (Server%20Name :type Text))
  ;[1 1 1] Initial Setup
  (Variables|Default|SetbShowMouseCursor true)
  (bind _returnvalue (UserInterface|CreateWidget "/Game/BoardgameInterface/Environment/WaitingRoom/WaitingRoom_W.WaitingRoom_W_C" 0 Server%20Name))
  (bind _output_get (Variables|Widgets|SetWaiting%20Room%20Menu _returnvalue))
  (UserInterface|Viewport|AddtoViewport _output_get 0)
  (Input|SetInputModeUIOnly self (Variables|Widgets|GetWaiting%20Room%20Menu) "DoNotLock"))

(event Custom|Add%20Player%20Info
  (params (Connected%20Users%20Info :type Array%20of%20User%20Info%20STR%20Structures))
  (bind _waiting_room_menu (Variables|Widgets|GetWaiting%20Room%20Menu))
  ;[1 1 1] Update Waiting Room Information
  (Variables|UserInfo|SetAll%20Connected%20Users Connected%20Users%20Info)
  (Utilities|IsValid _waiting_room_menu
    (:Is%20Valid
      (Default|ClearUserList _waiting_room_menu)
      (for _array_element (Variables|UserInfo|GetAll%20Connected%20Users)
        (Default|UpdateUserWindow (Variables|Widgets|GetWaiting%20Room%20Menu) _array_element)))))

(event Custom|Update%20Waiting%20Room%20Settings
  (params (Map%20Thumbnail :type Texture%202D%20Object%20Reference) (Map%20Name :type Text) (Map%20Time :type Text))
  (bind _waiting_room_menu (Variables|Widgets|GetWaiting%20Room%20Menu))
  ;[1 1 1] Update Waiting Room Information
  (Variables|/Game/BoardgameInterface/Environment/WaitingRoom/WaitingRoom_W.WaitingRoom_W_C|SetMap%20Thumbnail _waiting_room_menu Map%20Thumbnail)
  (Variables|/Game/BoardgameInterface/Environment/WaitingRoom/WaitingRoom_W.WaitingRoom_W_C|SetMap%20Name _waiting_room_menu Map%20Name)
  (Variables|/Game/BoardgameInterface/Environment/WaitingRoom/WaitingRoom_W.WaitingRoom_W_C|SetMap%20Time _waiting_room_menu Map%20Time))

(event Custom|Show%20Loading%20Screen
  ;[1 1 1] Loading Screen
  (Widget|RemovefromParent (Variables|Widgets|GetWaiting%20Room%20Menu))
  (bind _returnvalue (UserInterface|CreateWidget "/Game/BoardgameInterface/Core/LoadingScreen_W.LoadingScreen_W_C" self))
  (UserInterface|Viewport|AddtoViewport _returnvalue 0))

(event Custom|Update%20User%20Number
  (params (Current%20Users :type Integer) (Max%20Users :type Integer))
  (bind _waiting_room_menu (Variables|Widgets|GetWaiting%20Room%20Menu))
  ;[1 1 1] Update Waiting Room Information
  (Utilities|IsValid _waiting_room_menu
    (:Is%20Valid
      (Variables|/Game/BoardgameInterface/Environment/WaitingRoom/WaitingRoom_W.WaitingRoom_W_C|SetNumber%20of%20Users _waiting_room_menu (Utilities|Text|FormatText "{Current Players} of {Max Players}" (Utilities|Text|ToText(Integer) Current%20Users) (Utilities|Text|ToText(Integer) Max%20Users))))))

(event Custom|Kicked
  ;[1 1 1] End Session
  (Game|OpenLevel(byName) "FrontMenu")
  (|DestroySession self))

(event Custom|Update%20Available%20Characters
  (params (Available%20Characters :type Array%20of%20Booleans))
  ;[1 1 1] Update Player Options
  (Variables|UserInfo|SetAvailable%20Characters Available%20Characters)
  (Utilities|IsValid (Variables|Widgets|GetWaiting%20Room%20Menu)
    (:Is%20Valid
      (for (_array_element _array_index) (Variables|/Game/BoardgameInterface/Environment/WaitingRoom/PlayerSettings_W.PlayerSettings_W_C|GetCharacter%20Buttons (Variables|/Game/BoardgameInterface/Environment/WaitingRoom/WaitingRoom_W.WaitingRoom_W_C|GetPlayerSettings_W (Variables|Widgets|GetWaiting%20Room%20Menu)))
        (Widget|SetIsEnabled _array_element (not (Utilities|Array|Get(acopy) (Variables|UserInfo|GetAvailable%20Characters) _array_index)))))))

(event Custom|Assign%20Selected%20Character
  (params (Character%20ID :type Integer) (Character%20Image :type Texture%202D%20Object%20Reference))
  ;[1 1 1] Character Selection
  (Variables|UserInfo|SetPrevious%20Selection (Variables|UserInfo|GetSelected%20Character))
  (Variables|UserInfo|SetCharacter%20Image Character%20Image)
  (Variables|UserInfo|SetSelected%20Character Character%20ID)
  (CallFunction|CharacterCheck))

(event EventEndPlay
  (params (EndPlayReason :type EEndPlayReason%20Enum :default "Destroyed"))
  ;[1 1 1] End Session
  (|DestroySession self))

(fn ConstructionScript)

(fn SaveGameCheck
  (bind _returnvalue (SaveGame|DoesSaveGameExist (Variables|/Game/BoardgameInterface/Core/Framework/AppInstance_BP.AppInstance_BP_C|GetSave%20Slot%20Name (.AsApp%20Instance%20BP (Utilities|Casting|CastToAppInstance_BP (Game|GetGameInstance))))))
  (if _returnvalue
    (CallFunction|LoadGame)
    (CallFunction|SaveGame)
    (else
      (CallFunction|SaveGame))))

(fn LoadGame
  (bind _returnvalue (SaveGame|LoadGamefromSlot (Variables|/Game/BoardgameInterface/Core/Framework/AppInstance_BP.AppInstance_BP_C|GetSave%20Slot%20Name (.AsApp%20Instance%20BP (Utilities|Casting|CastToAppInstance_BP (Game|GetGameInstance))))))
  (Utilities|Struct|SetmembersinUserInfo_STR (Variables|UserInfo|GetUser%20Settings) (.PlayerName (Utilities|Struct|BreakUserInfo_STR (Variables|/Game/BoardgameInterface/Core/Framework/UserSaveGame.UserSaveGame_C|GetUser%20Info (.AsUser%20Save%20Game (Utilities|Casting|CastToUserSaveGame _returnvalue))))) (.PlayerImage (Utilities|Struct|BreakUserInfo_STR (Variables|/Game/BoardgameInterface/Core/Framework/UserSaveGame.UserSaveGame_C|GetUser%20Info (.AsUser%20Save%20Game (Utilities|Casting|CastToUserSaveGame _returnvalue)))))))

(fn SaveGame
  (Utilities|IsValid (Variables|Default|GetSave%20Game%20Ref)
    (:Is%20Valid
      _)
    (:Is%20Not%20Valid
      (bind _returnvalue (SaveGame|CreateSaveGameObject "/Game/BoardgameInterface/Core/Framework/UserSaveGame.UserSaveGame_C"))
      (Variables|Default|SetSave%20Game%20Ref _returnvalue)))
  (Variables|/Game/BoardgameInterface/Core/Framework/UserSaveGame.UserSaveGame_C|SetUser%20Info (Variables|Default|GetSave%20Game%20Ref) (Variables|UserInfo|GetUser%20Settings))
  (SaveGame|SaveGametoSlot (Variables|Default|GetSave%20Game%20Ref) (Variables|/Game/BoardgameInterface/Core/Framework/AppInstance_BP.AppInstance_BP_C|GetSave%20Slot%20Name (.AsApp%20Instance%20BP (Utilities|Casting|CastToAppInstance_BP (Game|GetGameInstance))))))

(fn CharacterCheck
  (bind _returnvalue (Game|GetGameMode))
  (bind _aswaiting_room_mode_bp (Utilities|Casting|CastToWaitingRoomMode_BP _returnvalue))
  (bind _available_characters (Variables|/Game/BoardgameInterface/Environment/WaitingRoom/Framework/WaitingRoomMode_BP.WaitingRoomMode_BP_C|GetAvailable%20Characters _aswaiting_room_mode_bp))
  (if (== (Variables|UserInfo|GetSelected%20Character) 0)
    (Utilities|Array|SetArrayElem (Variables|/Game/BoardgameInterface/Environment/WaitingRoom/Framework/WaitingRoomMode_BP.WaitingRoomMode_BP_C|GetAvailable%20Characters (.AsWaiting%20Room%20Mode%20BP (Utilities|Casting|CastToWaitingRoomMode_BP (Game|GetGameMode)))) (Variables|UserInfo|GetPrevious%20Selection) false)
    (CallFunction|AssignPlayer "No Character" (Variables|UserInfo|GetCharacter%20Image))
    (elif (not (not (Utilities|Array|Get(acopy) _available_characters (Variables|UserInfo|GetSelected%20Character))))
      (Utilities|Array|SetArrayElem _available_characters (Variables|UserInfo|GetSelected%20Character) true)
      (Utilities|Array|SetArrayElem _available_characters (Variables|UserInfo|GetPrevious%20Selection) false)
      (CallFunction|AssignPlayer "No Character" (Variables|UserInfo|GetCharacter%20Image)))))