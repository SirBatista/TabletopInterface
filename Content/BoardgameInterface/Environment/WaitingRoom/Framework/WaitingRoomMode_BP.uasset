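; Game mode for the board game's multiplayer waiting room, managing joining and leaving users, map settings, kicking and server travel to GameRoom.
; PostLogin registers each controller, initializes its lobby menu and respawns its pawn.
; AllUsersUpdate rebuilds the user list, pushes player and character availability to every controller, and sets CanStart from chosen character names.
; Logout frees the character slot and re-syncs, while SwapCharacter can respawn pawns.
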(event Custom|Swap%20Character
  (params (Player%20Controller :type Player%20Controller%20Object%20Reference) (Character%20Name :type String) (Changed%20Status :type Boolean))
  (bind _returnvalue (Pawn|GetControlledPawn Player%20Controller))
  ;[1 1 1] Swaps Character
  (if (not Changed%20Status)
    (Utilities|IsValid _returnvalue
      (:Is%20Valid
        (Actor|DestroyActor _returnvalue))
      (:Is%20Not%20Valid
        _))
    (bind _returnvalue_2 (Game|SpawnActorfromClass "/Game/BoardgameInterface/Environment/WaitingRoom/Framework/WaitingRoomPawn_BP.WaitingRoomPawn_BP_C" (Math|Transform|MakeTransform "0, 0, 0" "0, 0, 0" "1,1,1") "AlwaysSpawn" 0 0))
    (Pawn|Possess Player%20Controller _returnvalue_2)))

(event Custom|All%20Users%20Update
  ;[1 1 1] Update Info on All Connected Users
  (bind _output_get (Variables|ServerSettings|SetCurrent%20User%20Number (Utilities|Array|Length (Variables|Default|GetUser%20Controllers))))
  (if (> _output_get 0)
    (Utilities|Array|Clear (Variables|Default|GetConnected%20Users%20Info))
    (for _array_element (Variables|Default|GetUser%20Controllers)
      (Utilities|Array|Add (Variables|Default|GetConnected%20Users%20Info) (Variables|/Game/BoardgameInterface/Environment/WaitingRoom/Framework/WaitingRoomController_BP.WaitingRoomController_BP_C|GetUser%20Settings (.AsWaiting%20Room%20Controller%20BP (Utilities|Casting|CastToWaitingRoomController_BP _array_element))))
      (Default|UpdateUserNumber (.AsWaiting%20Room%20Controller%20BP (Utilities|Casting|CastToWaitingRoomController_BP _array_element)) (Variables|ServerSettings|GetCurrent%20User%20Number) (Variables|ServerSettings|GetUser%20Capacity)))
    (for _array_element_2 (Variables|Default|GetUser%20Controllers)
      (Default|AddPlayerInfo (.AsWaiting%20Room%20Controller%20BP (Utilities|Casting|CastToWaitingRoomController_BP _array_element_2)) (Variables|Default|GetConnected%20Users%20Info))
      (Default|UpdateAvailableCharacters (.AsWaiting%20Room%20Controller%20BP (Utilities|Casting|CastToWaitingRoomController_BP _array_element_2)) (Variables|ServerSettings|GetAvailable%20Characters))
      (CallFunction|AddtoKickList))
    (bind _array_element_3 (Utilities|Array|ForEachLoopwithBreak (Variables|Default|GetConnected%20Users%20Info) :!label _label)
      (:LoopBody
        (if (Utilities|Enum|Equal(Enum) (Utilities|Struct|BreakUserInfo_STR _array_element_3) "")
          (Variables|ServerSettings|SetCan%20Start? false)
          (goto _label Break)
          (else
            (Variables|ServerSettings|SetCan%20Start? true)))))))

(event Custom|Launch%20Session
  ;[1 1 1] Launch Game
  (switch string (Variables|ServerSettings|GetMap%20ID)
    (:Default
      (Development|ExecuteConsoleCommand "servertravel GameRoom" 0))))

(event Custom|Respawn%20Player
  (params (Player%20Controller :type Player%20Controller%20Object%20Reference))
  (bind _returnvalue (Pawn|GetControlledPawn Player%20Controller))
  ;[1 1 1] Assign Pawn
  (Utilities|IsValid _returnvalue
    (:Is%20Valid
      (Actor|DestroyActor _returnvalue)
      (bind _returnvalue_2 (Game|SpawnActorfromClass "/Game/BoardgameInterface/Environment/WaitingRoom/Framework/WaitingRoomPawn_BP.WaitingRoomPawn_BP_C" (Math|Transform|MakeTransform "0, 0, 0" "0, 0, 0" "1,1,1") "AlwaysSpawn" 0 0))
      (Pawn|Possess Player%20Controller _returnvalue_2)
      (CallFunction|AllUsersUpdate))))

(event Custom|Add%20to%20Kick%20List
  ;[1 1 1] Add a user to Kick List if they login while window is open.
  (bind _aswaiting_room_controller_bp (Utilities|Casting|CastToWaitingRoomController_BP (Game|GetPlayerController 0)))
  (Utilities|IsValid (Variables|/Game/BoardgameInterface/Environment/WaitingRoom/Framework/WaitingRoomController_BP.WaitingRoomController_BP_C|GetWaiting%20Room%20Menu _aswaiting_room_controller_bp)
    (:Is%20Valid
      (if (Widget|IsVisible (Variables|/Game/BoardgameInterface/Environment/WaitingRoom/WaitingRoom_W.WaitingRoom_W_C|GetSessionSettings_W (Variables|/Game/BoardgameInterface/Environment/WaitingRoom/Framework/WaitingRoomController_BP.WaitingRoomController_BP_C|GetWaiting%20Room%20Menu _aswaiting_room_controller_bp)))
        (Default|FillKickUserWindow (Variables|/Game/BoardgameInterface/Environment/WaitingRoom/WaitingRoom_W.WaitingRoom_W_C|GetSessionSettings_W (Variables|/Game/BoardgameInterface/Environment/WaitingRoom/Framework/WaitingRoomController_BP.WaitingRoomController_BP_C|GetWaiting%20Room%20Menu _aswaiting_room_controller_bp)))))))

(event Custom|Server%20Update%20Session%20Settings
  (params (Map%20Thumbnail :type Texture%202D%20Object%20Reference) (Map%20Name :type Text) (Map%20Time :type Text) (Map%20ID :type String))
  ;[1 1 1] Update Session Settings
  (Variables|ServerSettings|SetMap%20Thumbnail Map%20Thumbnail)
  (Variables|ServerSettings|SetMap%20Name Map%20Name)
  (Variables|ServerSettings|SetMap%20Time Map%20Time)
  (Variables|ServerSettings|SetMap%20ID Map%20ID)
  (for _array_element (Variables|Default|GetUser%20Controllers)
    (Default|UpdateWaitingRoomSettings (.AsWaiting%20Room%20Controller%20BP (Utilities|Casting|CastToWaitingRoomController_BP _array_element)) (Variables|ServerSettings|GetMap%20Thumbnail) (Variables|ServerSettings|GetMap%20Name) (Variables|ServerSettings|GetMap%20Time))))

(event Custom|Kick%20User
  (params (Player%20ID :type Integer))
  ;[1 1 1] Kick User
  (Default|Kicked (.AsWaiting%20Room%20Controller%20BP (Utilities|Casting|CastToWaitingRoomController_BP (Utilities|Array|Get(acopy) (Variables|Default|GetUser%20Controllers) Player%20ID)))))

(event EventPostLogin
  (params (NewPlayer :type Player%20Controller%20Object%20Reference))
  ;[1 1 1] Incoming Player Setup
  (Networking|SwitchHasAuthority
    (:Authority
      (Utilities|Array|Add (Variables|Default|GetUser%20Controllers) NewPlayer)
      (bind _asapp_instance_bp (Utilities|Casting|CastToAppInstance_BP (Game|GetGameInstance)))
      (Variables|ServerSettings|SetServer%20Name (Variables|/Game/BoardgameInterface/Core/Framework/AppInstance_BP.AppInstance_BP_C|GetServer%20Name _asapp_instance_bp))
      (Variables|ServerSettings|SetUser%20Capacity (Variables|/Game/BoardgameInterface/Core/Framework/AppInstance_BP.AppInstance_BP_C|GetUser%20Capacity _asapp_instance_bp))
      (bind _aswaiting_room_controller_bp (Utilities|Casting|CastToWaitingRoomController_BP NewPlayer))
      (Default|SetupLobbyMenu _aswaiting_room_controller_bp (Variables|ServerSettings|GetServer%20Name))
      (Default|InitialSetup _aswaiting_room_controller_bp)
      (Default|UpdateWaitingRoomSettings _aswaiting_room_controller_bp (Variables|ServerSettings|GetMap%20Thumbnail) (Variables|ServerSettings|GetMap%20Name) (Variables|ServerSettings|GetMap%20Time))
      (CallFunction|RespawnPlayer _aswaiting_room_controller_bp))))

(event EventOnLogout
  (params (ExitingController :type Controller%20Object%20Reference))
  ;[1 1 1] Event On Logout
  (bind (_array_element _array_index) (Utilities|Array|ForEachLoopwithBreak (Variables|Default|GetUser%20Controllers) :!label _label)
    (:LoopBody
      (if (== _array_element ExitingController)
        (Variables|ServerSettings|SetLogout%20User%20Index _array_index)
        (goto _label Break)))
    (:Completed
      (bind _aswaiting_room_controller_bp (Utilities|Casting|CastToWaitingRoomController_BP (Utilities|Array|Get(acopy) (Variables|Default|GetUser%20Controllers) (Variables|ServerSettings|GetLogout%20User%20Index))))
      (Utilities|Array|SetArrayElem (Variables|ServerSettings|GetAvailable%20Characters) (Variables|/Game/BoardgameInterface/Environment/WaitingRoom/Framework/WaitingRoomController_BP.WaitingRoomController_BP_C|GetSelected%20Character _aswaiting_room_controller_bp) false)
      (Utilities|Array|RemoveIndex (Variables|Default|GetUser%20Controllers) (Variables|ServerSettings|GetLogout%20User%20Index))
      (Utilities|Array|RemoveIndex (Variables|Default|GetConnected%20Users%20Info) (Variables|ServerSettings|GetLogout%20User%20Index))
      (CallFunction|AllUsersUpdate))))

(fn ConstructionScript)