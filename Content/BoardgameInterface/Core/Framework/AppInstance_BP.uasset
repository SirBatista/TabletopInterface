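; Game instance for a board game interface that manages app-level menus, the loading screen and multiplayer sessions.
; Menu events create and display widgets, caching most for reuse, and a save-game check opens either the main menu or first-time settings.
; Hosting creates a session and opens WaitingRoom as a listen server, while joining uses a search result.
; Session failures and network or travel errors become readable messages passed to an error dialogue widget.
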(event Custom|Show%20Main%20Menu
  (bind _returnvalue (Game|GetPlayerController 0))
  ;[1 1 1] Window Manager
  (Utilities|IsValid (Variables|Widgets|GetApp%20Menu)
    (:Is%20Valid
      _)
    (:Is%20Not%20Valid
      (bind _returnvalue_2 (UserInterface|CreateWidget "/Game/BoardgameInterface/Environment/AppMenu/AppMenu_W.AppMenu_W_C" _returnvalue))
      (Variables|Widgets|SetApp%20Menu _returnvalue_2)))
  (UserInterface|Viewport|AddtoViewport (Variables|Widgets|GetApp%20Menu) 0)
  (Variables|/Script/Engine.PlayerController|SetbShowMouseCursor _returnvalue true))

(event Custom|Show%20Hosting%20Menu
  (bind _returnvalue (Game|GetPlayerController 0))
  ;[1 1 1] Window Manager
  (Utilities|IsValid (Variables|Widgets|GetHosting%20Menu)
    (:Is%20Valid
      _)
    (:Is%20Not%20Valid
      (bind _returnvalue_2 (UserInterface|CreateWidget "/Game/BoardgameInterface/Environment/AppMenu/HostingMenu_W.HostingMenu_W_C" _returnvalue))
      (Variables|Widgets|SetHosting%20Menu _returnvalue_2)))
  (UserInterface|Viewport|AddtoViewport (Variables|Widgets|GetHosting%20Menu) 0)
  (Variables|/Script/Engine.PlayerController|SetbShowMouseCursor _returnvalue true))

(event Custom|Show%20Server%20Menu
  ;[1 1 1] Window Manager
  (bind _returnvalue (UserInterface|CreateWidget "/Game/BoardgameInterface/Environment/AppMenu/ServerListMenu_W.ServerListMenu_W_C" (Game|GetPlayerController 0)))
  (UserInterface|Viewport|AddtoViewport _returnvalue 0))

(event Custom|Show%20Settings%20Menu
  (bind _returnvalue (Game|GetPlayerController 0))
  ;[1 1 1] Window Manager
  (Utilities|IsValid (Variables|Widgets|GetSettings%20Menu)
    (:Is%20Valid
      _)
    (:Is%20Not%20Valid
      (bind _returnvalue_2 (UserInterface|CreateWidget "/Game/BoardgameInterface/Environment/AppMenu/SettingsMenu_W.SettingsMenu_W_C" _returnvalue))
      (Variables|Widgets|SetSettings%20Menu _returnvalue_2)))
  (UserInterface|Viewport|AddtoViewport (Variables|Widgets|GetSettings%20Menu) 0)
  (Variables|/Script/Engine.PlayerController|SetbShowMouseCursor _returnvalue true)
  (if (not (Variables|Default|GetCreated%20Save%20File?))
    (Variables|/Game/BoardgameInterface/Environment/AppMenu/SettingsMenu_W.SettingsMenu_W_C|SetWelcome%20Message%20Visibility (Variables|Widgets|GetSettings%20Menu) "Visible")))

(event Custom|Launch%20Lobby
  (params (User%20Capacity :type Integer) (Enable%20LAN :type Boolean) (Server%20Name :type Text))
  ;[1 1 1] Session Management
  (Variables|ServerSettings|SetUser%20Capacity User%20Capacity)
  (Variables|ServerSettings|SetServer%20Name Server%20Name)
  (CallFunction|ShowLoadingScreen)
  (|Session (Game|GetPlayerController 0) (Variables|ServerSettings|GetUser%20Capacity) Enable%20LAN
    (:OnSuccess
      (Game|OpenLevel(byName) "WaitingRoom" true "listen"))
    (:OnFailure
      (Utilities|ErrorReport "Failed to create session. Please try again."))))

(event Custom|Show%20Loading%20Screen
  (bind _returnvalue (Game|GetPlayerController 0))
  ;[1 1 1] Window Manager
  (Utilities|IsValid (Variables|Widgets|GetLoading%20Screen)
    (:Is%20Valid
      _)
    (:Is%20Not%20Valid
      (bind _returnvalue_2 (UserInterface|CreateWidget "/Game/BoardgameInterface/Core/LoadingScreen_W.LoadingScreen_W_C" _returnvalue))
      (Variables|Widgets|SetLoading%20Screen _returnvalue_2)))
  (UserInterface|Viewport|AddtoViewport (Variables|Widgets|GetLoading%20Screen) 0)
  (Variables|/Script/Engine.PlayerController|SetbShowMouseCursor _returnvalue false))

(event Custom|Join%20Server
  (params (Session :type Blueprint%20Session%20Result%20Structure))
  ;[1 1 1] Session Management
  (CallFunction|ShowLoadingScreen)
  (|JoinSession (Game|GetPlayerController 0) Session
    (:OnFailure
      (Utilities|ErrorReport "Failed to join session. Please try again."))))

(event Custom|Destroy%20Session%20Caller
  (params (Controller :type Player%20Controller%20Object%20Reference))
  ;[1 1 1] Session Management
  (|DestroySession Controller))

(event Custom|Save%20Game%20Check
  ;[1 1 1] Save Game Check
  (bind _returnvalue (SaveGame|DoesSaveGameExist (Variables|Default|GetSave%20Slot%20Name)))
  (if _returnvalue
    (CallFunction|ShowMainMenu)
    (Variables|Default|SetCreated%20Save%20File? true)
    (else
      (CallFunction|ShowSettingsMenu))))

(event EventHandleNetworkError
  (params (FailureType :type ENetworkFailure%20Enum :default "NetDriverAlreadyExists") (bIsServer :type Boolean))
  ;[1 1 1] Session Management
  (Utilities|ErrorReport (CallFunction|NetworkErrortoVerbose FailureType)))

(event EventHandleTravelError
  (params (FailureType :type ETravelFailure%20Enum :default "NoLevel"))
  ;[1 1 1] Session Management
  (Utilities|ErrorReport (CallFunction|TravelErrortoVerbose FailureType)))

(fn NetworkErrortoVerbose
  (params (Error :type ENetworkFailure%20Enum :default "NetDriverAlreadyExists"))
  (switch Utilities|FlowControl|Switch|SwitchonENetworkFailure Error
    (:NetDriverAlreadyExists
      _)
    (:NetDriverCreateFailure
      _)
    (:NetDriverListenFailure
      _)
    (:ConnectionLost
      _)
    (:ConnectionTimeout
      (return "Connection timed out."))
    (:FailureReceived
      _)
    (:OutdatedClient
      (return "Outdated connection."))
    (:OutdatedServer
      (return "Outdated connection."))
    (:PendingConnectionFailure
      _)
    (:NetGuidMismatch
      _)
    (:NetChecksumMismatch
      _))
  (return "Lost connection to host."))

(fn TravelErrortoVerbose
  (params (Error :type ETravelFailure%20Enum :default "NoLevel"))
  (return (Utilities|String|Append "Failed to travel." (Utilities|String|EnumtoString Error))))